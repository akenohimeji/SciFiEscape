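; BP_Target is a damageable target actor that reacts physically and visually to hits.
; On any damage, its Cube receives an impulse along the player camera's forward vector, applied at world origin, and briefly swaps to a hit material.
; After the short delay it restores the normal material and destroys itself if Health is zero or below.
; The Health subtraction uses a constant zero, so damage never lowers it.
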(event EventBeginPlay)

(event Collision|EventActorBeginOverlap
  (params (OtherActor :type Actor%20Object%20Reference)))

(event EventTick
  (params (DeltaSeconds :type Float%20%28single-precision%29)))

(event Game|Damage|EventAnyDamage
  (params (Damage :type Float%20%28single-precision%29) (DamageType :type Damage%20Type%20Object%20Reference) (InstigatedBy :type Controller%20Object%20Reference) (DamageCauser :type Actor%20Object%20Reference))
  (Physics|AddImpulseatLocation (Variables|Default|GetCube) (* (Transformation|GetActorForwardVector (Game|GetPlayerCameraManager 0)) 5e+04) "0, 0, 0" "None")
  (Rendering|Material|SetMaterial (Variables|Default|GetCube) 0 "/Game/Actors/M_TargetHit.M_TargetHit")
  (Utilities|FlowControl|Delay 0.1)
  (Rendering|Material|SetMaterial (Variables|Default|GetCube) 0 "/Game/Actors/M_TargetNormal.M_TargetNormal")
  (bind _output_get (Variables|Default|SetHealth (- (Variables|Default|GetHealth) 0.0)))
  (if (<= _output_get 0.0)
    (Actor|DestroyActor)))

(fn ConstructionScript)